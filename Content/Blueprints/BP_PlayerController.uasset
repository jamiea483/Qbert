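; BP_PlayerController is a player controller that routes menu input to the pause menu.
; The UpLeft and DownRight actions call MenuControl with opposite step directions, and Enter calls SelectionControl.
; Each input acts only while GamePaused is true and the PauseMenu reference is valid.
; The graph only reads those two variables and does not set them.
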(event Input|ActionEvents|InputActionUpLeft
  (params (Key :type Key%20Structure :default "None"))
  (bind _pausemenu (Variables|Default|GetpauseMenu))
  (:Pressed
    (if (Variables|Default|GetbGamePaused)
      (Utilities|IsValid _pausemenu
        (:Is%20Valid
          (Default|MenuControl _pausemenu -1))))))

(event Input|ActionEvents|InputActionDownRight
  (params (Key :type Key%20Structure :default "None"))
  (bind _pausemenu (Variables|Default|GetpauseMenu))
  (:Pressed
    (if (Variables|Default|GetbGamePaused)
      (Utilities|IsValid _pausemenu
        (:Is%20Valid
          (Default|MenuControl _pausemenu 1))))))

(event Input|ActionEvents|InputActionEnter
  (params (Key :type Key%20Structure :default "None"))
  (bind _pausemenu (Variables|Default|GetpauseMenu))
  (:Pressed
    (if (Variables|Default|GetbGamePaused)
      (Utilities|IsValid _pausemenu
        (:Is%20Valid
          (Default|SelectionControl _pausemenu))))))

(fn ConstructionScript)