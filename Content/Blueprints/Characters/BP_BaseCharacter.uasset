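; Base character for a Q*bert-style game that hops diagonally between tiles on a tile map.
; Four move functions, gated on IsGrounded, step the tile X or Y coordinate and apply a capsule impulse, stronger upward for upward hops.
; TranslateQBert lerps the actor toward that tile's corner position by JumpTime at a fixed Y depth.
; It sets IsGrounded when the actor is not within tolerance of that target.
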(fn ConstructionScript)

(fn MoveDownRight
  (if (Variables|Default|GetIsGrounded)
    (bind _result (Math|Integer|IncrementInt (Math|Float|Truncate (.X (Math|Vector|BreakVector (Variables|Default|GetTileLocation)))))
      (:%20%20
        (Variables|Default|SetTileLocation (Math|Vector|MakeVector (Math|Conversions|ToFloat(Integer) _result) (.Y (Math|Vector|BreakVector (Variables|Default|GetTileLocation))) (.Z (Math|Vector|BreakVector (Variables|Default|GetTileLocation)))))
        (Physics|AddImpulse (Variables|Collision|GetCapsuleComponent) "100.000000,15.000000,100.000000" "None" false)))))

(fn MoveUpLeft
  (if (Variables|Default|GetIsGrounded)
    (bind _result (Math|Integer|DecrementInt (Math|Float|Truncate (.X (Math|Vector|BreakVector (Variables|Default|GetTileLocation)))))
      (:%20%20
        (Variables|Default|SetTileLocation (Math|Vector|MakeVector (Math|Conversions|ToFloat(Integer) _result) (.Y (Math|Vector|BreakVector (Variables|Default|GetTileLocation))) (.Z (Math|Vector|BreakVector (Variables|Default|GetTileLocation)))))
        (Physics|AddImpulse (Variables|Collision|GetCapsuleComponent) "-80.000000,-15.000000,450.000000" "None" false)))))

(fn MoveDownLeft
  (if (Variables|Default|GetIsGrounded)
    (bind _result (Math|Integer|IncrementInt (Math|Float|Truncate (.Y (Math|Vector|BreakVector (Variables|Default|GetTileLocation)))))
      (:%20%20
        (Variables|Default|SetTileLocation (Math|Vector|MakeVector (.X (Math|Vector|BreakVector (Variables|Default|GetTileLocation))) (Math|Conversions|ToFloat(Integer) _result) (.Z (Math|Vector|BreakVector (Variables|Default|GetTileLocation)))))
        (Physics|AddImpulse (Variables|Collision|GetCapsuleComponent) "-100.000000,15.000000,100.000000" "None" false)))))

(fn MoveUpRight
  (if (Variables|Default|GetIsGrounded)
    (bind _result (Math|Integer|DecrementInt (Math|Float|Truncate (.Y (Math|Vector|BreakVector (Variables|Default|GetTileLocation)))))
      (:%20%20
        (Variables|Default|SetTileLocation (Math|Vector|MakeVector (.X (Math|Vector|BreakVector (Variables|Default|GetTileLocation))) (Math|Conversions|ToFloat(Integer) _result) (.Z (Math|Vector|BreakVector (Variables|Default|GetTileLocation)))))
        (Physics|AddImpulse (Variables|Collision|GetCapsuleComponent) "80.000000,-15.000000,450.000000" "None" false)))))

(fn TranslateQBert
  (bind _self self)
  (bind _newvar_1 (Variables|Default|GetNewVar_1))
  (bind _tilelocation (Variables|Default|GetTileLocation))
  (bind (_x _y) (Math|Vector|BreakVector _tilelocation))
  (bind _returnvalue (Transformation|GetActorLocation _self))
  (bind _rendercomponent (Variables|/Script/Paper2D.PaperTileMapActor|GetRenderComponent _newvar_1))
  (bind _returnvalue_2 (Math|Float|Truncate _x))
  (bind _returnvalue_3 (Math|Float|Truncate _y))
  (bind _returnvalue_4 (Class|PaperTileMapComponent|GetTileCornerPosition _rendercomponent _returnvalue_2 _returnvalue_3 0 false))
  (bind (_x_2 _y_2 _z) (Math|Vector|BreakVector _returnvalue_4))
  (bind _returnvalue_5 (- _z 15.0))
  (bind _returnvalue_6 (Math|Vector|MakeVector _x_2 0.1 _returnvalue_5))
  (Transformation|SetActorLocation (Math|Vector|Lerp(Vector) _returnvalue _returnvalue_6 (Variables|Default|GetJumpTime)) false false)
  (if (not (Math|Vector|Equal(Vector) _returnvalue _returnvalue_6 1.0))
    (Variables|Default|SetIsGrounded true)))