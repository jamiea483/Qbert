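; Enemy pawn for a Q*bert-style game, acting as either a random green or red slime or a snake.
; Tick runs a movement timer that triggers grounded hops with type-specific sounds, resetting to an interval shortened by game level.
; Until SetGrown is called, enemies hop randomly down-left or down-right.
; Grown enemies compare positions with the player and hop diagonally toward them, swapping snake flipbooks by direction.
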(event EventBeginPlay
  (bind _asqbert_game_mode (Utilities|Casting|CastToQbertGameMode (Game|GetGameMode)))
  (Variables|Default|SetGM _asqbert_game_mode)
  (switch Utilities|FlowControl|Switch|SwitchonE_EnemyType (Variables|Default|GetEnemyType)
    (:NewEnumerator0
      (if (== (Math|Random|RandomInteger 2) 1)
        (Sprite|SetFlipbook (Variables|Default|GetSprite) "/Game/Blueprints/Characters/Enemys/Sprites/Slimes/FB_GreenSlime.FB_GreenSlime")
        (else
          (Sprite|SetFlipbook (Variables|Default|GetSprite) "/Game/Blueprints/Characters/Enemys/Sprites/Slimes/FB_RedSlime.FB_RedSlime"))))
    (:NewEnumerator1
      (Sprite|SetFlipbook (Variables|Default|GetSprite) "/Game/Blueprints/Characters/Enemys/Sprites/Snake/BabySnake.BabySnake")
      (bind _outactors (Actor|GetAllActorsOfClass "/Game/Blueprints/Characters/Player/Qbert/BP_Player.BP_Player_C"))
      (Utilities|IsValid (Utilities|Array|Get(acopy) _outactors)
        (:Is%20Valid
          (Variables|Default|SetPlayerRef (Utilities|Array|Get(acopy) _outactors)))))))

(event EventTick
  (params (DeltaSeconds :type Float%20%28single-precision%29))
  (|CallParentFunction DeltaSeconds)
  (if (Variables|Default|GetbIsGrown)
    (if (Variables|Default|GetIsGrounded)
      (bind _output_get (Variables|Default|SetMovementTimer (- (Variables|Default|GetMovementTimer) (* DeltaSeconds (Math|Float|MakeLiteralFloat 1.0)))))
      (if (<= _output_get 0.0)
        (Utilities|FlowControl|DoOnce false :!label _label
          (:Completed
            (Utilities|IsValid (Variables|Default|GetPlayerRef)
              (:Is%20Valid
                (CallFunction|UpdatePlayerLocation (Variables|Default|GetPlayerRef))
                (CallFunction|SnakeMovement)
                (CallFunction|SoundEffects)
                (CallFunction|EnemyMovementTimer)
                (goto _label Reset)))))
        (else
          (goto _label_2 Reset)))
      (else
        (Utilities|FlowControl|DoOnce false :!label _label_2
          (:Completed
            (CallFunction|EnemyMovementTimer)))))
    (else
      (Variables|Default|SetMovementTimer (- (Variables|Default|GetMovementTimer) (* DeltaSeconds (Math|Float|MakeLiteralFloat 1.0))))
      (if (Variables|Default|GetIsGrounded)
        (bind _output_get_2 (Variables|Default|SetMovementTimer (- (Variables|Default|GetMovementTimer) (* DeltaSeconds (Math|Float|MakeLiteralFloat 1.0)))))
        (if (<= _output_get_2 0.0)
          (Utilities|FlowControl|DoOnce false :!label _label_3
            (:Completed
              (CallFunction|SlimeMovement)
              (CallFunction|SoundEffects)
              (CallFunction|EnemyMovementTimer)
              (goto _label_3 Reset)))
          (else
            (goto _label_4 Reset)))
        (else
          (Utilities|FlowControl|DoOnce false :!label _label_4
            (:Completed
              (CallFunction|EnemyMovementTimer))))))))

(fn ConstructionScript
  (|CallParentFunction))

(fn SlimeMovement
  (if (Variables|Default|GetIsGrounded)
    (if (< (Math|Random|RandomInteger 2) 1)
      (CallFunction|MoveDownLeft)
      (else
        (CallFunction|MoveDownRight)))))

(fn SnakeMovement
  (if (and (< (Variables|Default|GetPlayerXLocation) (Variables|Default|GetSelfXLocation)) (> (Variables|Default|GetPlayerZLocation) (Variables|Default|GetSelfZLocation)))
    (CallFunction|MoveUpLeft)
    (Sprite|SetFlipbook (Variables|Default|GetSprite) "/Game/Blueprints/Characters/Enemys/Sprites/Snake/FB_Snake_UpLeft.FB_Snake_UpLeft")
    (elif (and (> (Variables|Default|GetPlayerXLocation) (Variables|Default|GetSelfZLocation)) (> (Variables|Default|GetPlayerZLocation) (Variables|Default|GetSelfZLocation)))
      (CallFunction|MoveUpRight)
      (Sprite|SetFlipbook (Variables|Default|GetSprite) "/Game/Blueprints/Characters/Enemys/Sprites/Snake/FB_Snake_UpRight.FB_Snake_UpRight")
      (elif (and (> (Variables|Default|GetPlayerXLocation) (Variables|Default|GetSelfXLocation)) (< (Variables|Default|GetPlayerZLocation) (Variables|Default|GetSelfZLocation)))
        (CallFunction|MoveDownRight)
        (Sprite|SetFlipbook (Variables|Default|GetSprite) "/Game/Blueprints/Characters/Enemys/Sprites/Snake/FB_Snake_DownRight.FB_Snake_DownRight")
        (elif (and (< (Variables|Default|GetPlayerXLocation) (Variables|Default|GetSelfXLocation)) (< (Variables|Default|GetPlayerZLocation) (Variables|Default|GetSelfZLocation)))
          (CallFunction|MoveDownLeft)
          (Sprite|SetFlipbook (Variables|Default|GetSprite) "/Game/Blueprints/Characters/Enemys/Sprites/Snake/FB_Snake_DownLeft.FB_Snake_DownLeft"))))))

(fn UpdatePlayerLocation
  (params (self2 :type Actor%20Object%20Reference))
  (bind _returnvalue (Transformation|GetActorLocation))
  (bind _returnvalue_2 (Transformation|GetActorLocation self2))
  (bind (_x _y _z) (Math|Vector|BreakVector _returnvalue_2))
  (bind (_x_2 _y_2 _z_2) (Math|Vector|BreakVector _returnvalue))
  (Variables|Default|SetPlayerXLocation _x)
  (Variables|Default|SetPlayerZLocation _z)
  (Variables|Default|SetSelfXLocation _x_2)
  (Variables|Default|SetSelfZLocation _z_2))

(fn SoundEffects
  (switch Utilities|FlowControl|Switch|SwitchonE_EnemyType (Variables|Default|GetEnemyType)
    (:NewEnumerator0
      (CallFunction|Jumped (LocalVariables|GetLocalSlimeSFX)))
    (:NewEnumerator1
      (CallFunction|Jumped (LocalVariables|GetLocalSnakeSFX)))))

(fn EnemyMovementTimer
  (bind _resettimer (Variables|Default|GetResetTimer))
  (Variables|Default|SetMovementTimer (Math|Float|Clamp(Float) _resettimer 1.0 (- _resettimer (* (Default|GetLevel (Variables|Default|GetGM)) 0.5)))))

(fn SetGrown
  (Variables|Default|SetbIsGrown true))