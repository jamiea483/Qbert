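; Enemy spawner actor that spawns BP_Enemy of a configured type, Slime or Snake, at its own transform.
; CanSpawnEnemy counts down a timer while playing and spawns when it expires and the count passes that type's limit check.
; Each spawn passes the type and spawner reference, increments the count and restarts the timer.
; When play is inactive, a DoOnce, re-armed by each spawn, resets the timer.
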(event Custom|CanSpawnEnemy
  (params (DeltaTime :type Float%20%28single-precision%29) (IsPlaying :type Boolean))
  (if IsPlaying
    (Variables|Default|SetSpawnTimer (- (Variables|Default|GetSpawnTimer) DeltaTime))
    (bind _returnvalue (CallFunction|AtSpawnLimt))
    (if _returnvalue
      (if (<= (Variables|Default|GetSpawnTimer) 0.0)
        (Game|SpawnActorfromClass "/Game/Blueprints/Characters/Enemys/BP_Enemy.BP_Enemy_C" (Transformation|GetActorTransform) "Undefined" 0 (Variables|Default|GetTypeToSpawn) self 0)
        (bind _result (Math|Integer|IncrementInt (Variables|Default|GetEnemyLimit))
          (:%20%20
            (Variables|Default|SetEnemyLimit _result)
            (Variables|Default|SetSpawnTimer (Variables|Default|GetTimeToResetTimeTo))
            (goto _label Reset)))))
    (else
      (Utilities|FlowControl|DoOnce false :!label _label
        (:Completed
          (Variables|Default|SetSpawnTimer (Variables|Default|GetTimeToResetTimeTo)))))))

(fn ConstructionScript)

(fn AtSpawnLimt
  (switch Utilities|FlowControl|Switch|SwitchonE_EnemyType (Variables|Default|GetTypeToSpawn)
    (:NewEnumerator0
      (Variables|Default|SetbCanSpawn (<= (Variables|Default|GetEnemyLimit) (Variables|Default|GetMaxSlimeEnemys))))
    (:NewEnumerator1
      (Variables|Default|SetbCanSpawn (<= (Variables|Default|GetEnemyLimit) (Variables|Default|GetMaxSnakeEnemy)))))
  (return (Variables|Default|GetbCanSpawn)))