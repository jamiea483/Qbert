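; BP_Player is the player-controlled Qbert character, which hops in four diagonal directions.
; Each directional input calls a movement function defined outside this graph, swaps the sprite flipbook to face that way and plays a jump sound.
; BeginPlay caches the QbertGameMode, and a capsule overlap with any actor tagged Enemy tells it to restart the current level.
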(event OnComponentBeginOverlap(CapsuleComponent)
  (params (OverlappedComponent :type Primitive%20Component%20Object%20Reference) (OtherActor :type Actor%20Object%20Reference) (OtherComp :type Primitive%20Component%20Object%20Reference) (OtherBodyIndex :type Integer) (bFromSweep :type Boolean) (SweepResult :type Hit%20Result%20Structure%20%28by%20ref%29))
  (if (Actor|ActorHasTag OtherActor "Enemy")
    (Default|RestartCurrentLevel (Variables|Default|GetGM))))

(event EventBeginPlay
  (bind _asqbert_game_mode (Utilities|Casting|CastToQbertGameMode (Game|GetGameMode)))
  (Variables|Default|SetGM _asqbert_game_mode))

(event Input|ActionEvents|InputActionDownLeft
  (params (Key :type Key%20Structure :default "None"))
  (:Pressed
    (CallFunction|MoveDownLeft)
    (Sprite|SetFlipbook (Variables|Default|GetSprite) "/Game/Blueprints/Characters/Player/Qbert/Sprites/FB_Qbert_DownLeft.FB_Qbert_DownLeft")
    (Audio|PlaySound2D "/Game/Sounds/386613__jalastram__sfx-jump-02.386613__jalastram__sfx-jump-02" 1.0 1.0 0.0 0 0)))

(event Input|ActionEvents|InputActionDownRight
  (params (Key :type Key%20Structure :default "None"))
  (:Pressed
    (CallFunction|MoveDownRight)
    (Sprite|SetFlipbook (Variables|Default|GetSprite) "/Game/Blueprints/Characters/Player/Qbert/Sprites/FB_Qbert_DownRight.FB_Qbert_DownRight")
    (Audio|PlaySound2D "/Game/Sounds/386613__jalastram__sfx-jump-02.386613__jalastram__sfx-jump-02" 1.0 1.0 0.0 0 0)))

(event Input|ActionEvents|InputActionUpLeft
  (params (Key :type Key%20Structure :default "None"))
  (:Pressed
    (CallFunction|MoveUpLeft)
    (Sprite|SetFlipbook (Variables|Default|GetSprite) "/Game/Blueprints/Characters/Player/Qbert/Sprites/FB_Qbert_UpLeft.FB_Qbert_UpLeft")
    (Audio|PlaySound2D "/Game/Sounds/386613__jalastram__sfx-jump-02.386613__jalastram__sfx-jump-02" 1.0 1.0 0.0 0 0)))

(event Input|ActionEvents|InputActionUpRight
  (params (Key :type Key%20Structure :default "None"))
  (:Pressed
    (CallFunction|MoveUpRight)
    (Sprite|SetFlipbook (Variables|Default|GetSprite) "/Game/Blueprints/Characters/Player/Qbert/Sprites/FB_Qbert_upright.FB_Qbert_upright")
    (Audio|PlaySound2D "/Game/Sounds/386613__jalastram__sfx-jump-02.386613__jalastram__sfx-jump-02" 1.0 1.0 0.0 0 0)))

(fn ConstructionScript
  (|CallParentFunction))