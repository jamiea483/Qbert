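; Game mode for a Q*bert-style game, running levels, rounds, lives and game over.
; Tick counts down the splash screen, advances rounds when all platforms are finished, and spawns snakes before slimes up to per-type caps.
; Each round change shows the splash, rebuilds the level through BP_LevelMaker with cycling sprite sets, and respawns the player afterwards.
; Deaths clear enemies and cost a life, leading to respawn or game over.
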(event Custom|UpdateScore
  ;[1 1 1] Update Score
  (Default|UpdateScore (Variables|Default|GetGameUI)))

(event Custom|LevelUpdate
  (bind _levelmaker (Variables|Default|GetLevelMaker))
  (Default|ClearLevel _levelmaker)
  (Default|MakeLevel _levelmaker)
  ;[1 1 1] Set All Platform Sprites to the base sprite for the level
  (for _array_element (Variables|/Game/Blueprints/Platform/BP_LevelMaker.BP_LevelMaker_C|GetPlatformArray _levelmaker)
    (Rendering|Components|Sprite|SetSprite (Variables|/Game/Blueprints/Platform/BP_Platform.BP_Platform_C|GetPaperSprite _array_element) (Utilities|Array|Get(acopy) (Variables|Default|GetLevelSprites) (* (Math|Integer|%(Integer) (Variables|Default|GetLevel) 3) 4)))
    ;[0 0.07465 1] ChangeTo
    (Default|UpdateChangeto (Variables|Default|GetGameUI) (Utilities|Array|Get(acopy) (Variables|Default|GetLevelSprites) (+ (* (Math|Integer|%(Integer) (Variables|Default|GetLevel) 3) 4) (Variables|Default|GetRound))))
    (Default|UpdateLevel (Variables|Default|GetGameUI) (+ (Variables|Default|GetLevel) 1))
    (Default|UpdateRound (Variables|Default|GetGameUI) (Variables|Default|GetRound))))

(event Custom|RestartCurrentLevel
  (Utilities|FlowControl|DoOnce false :!label _label
    (:Completed
      (bind _newparam (CallFunction|CharacterDie false))
      (Utilities|FlowControl|Delay 2.0)
      (if _newparam
        (bind _returnvalue (UserInterface|CreateWidget "/Game/UI/WBP_GameOver.WBP_GameOver_C"))
        (UserInterface|Viewport|AddtoViewport _returnvalue 0)
        (CallFunction|CharacterDie false)
        (else
          (CallFunction|SpawnPlayer)
          (goto _label Reset))))))

(event EventBeginPlay
  (bind _returnvalue (UserInterface|CreateWidget "/Game/UI/WBP_GameUI.WBP_GameUI_C" (Game|GetPlayerController 0)))
  (Variables|Default|SetGameUI _returnvalue)
  (UserInterface|Viewport|AddtoViewport _returnvalue 0)
  (bind _outactors (Actor|GetAllActorsOfClass "/Game/Blueprints/Platform/BP_LevelMaker.BP_LevelMaker_C"))
  (Variables|Default|SetLevelMaker (Utilities|Array|Get(acopy) _outactors))
  (bind _outactors_2 (Actor|GetAllActorsOfClass "/Game/Blueprints/Characters/Enemys/BP_EnemySpawner.BP_EnemySpawner_C"))
  (Variables|Default|SetSpawner _outactors_2)
  (CallFunction|DisplaySplashUI)
  (bind _outactors_3 (Actor|GetAllActorsOfClass "/Script/Engine.CameraActor"))
  (Variables|Default|SetLevelCamera (Utilities|Array|Get(acopy) _outactors_3))
  (Default|UpdateHiScore (Variables|Default|GetGameUI)))

(event EventTick
  (params (DeltaSeconds :type Float%20%28single-precision%29))
  (bind _returnvalue (Math|Random|RandomInteger 1))
  (bind _returnvalue_2 (Math|Float|MakeLiteralFloat 1.0))
  (bind _playerref (Variables|Default|GetPlayerRef))
  (bind _spawner (Variables|Default|GetSpawner))
  (bind _returnvalue_3 (* DeltaSeconds _returnvalue_2))
  (bind _output (Utilities|Array|Get(acopy) _spawner _returnvalue))
  ;[1 1 1] GameLoop
  (bind _outactors (Actor|GetAllActorsOfClass "/Game/Blueprints/Characters/BP_BaseCharacter.BP_BaseCharacter_C"))
  (Variables|Default|SetCharacters _outactors)
  (if (Variables|Default|GetbIsSplashScreenShowing)
    (Variables|Default|SetSplashScreenTimer (- (Variables|Default|GetSplashScreenTimer) _returnvalue_3))
    (else
      (Utilities|IsValid _playerref
        (:Is%20Valid
          (Default|SetJumpTimer _playerref _returnvalue_3 (Variables|Default|GetbIsPlaying))))))
  (Utilities|FlowControl|Sequence
    (:then_0
      (if (Variables|Default|GetbIsSplashScreenShowing)
        (if (<= (Variables|Default|GetSplashScreenTimer) 0.0)
          (CallFunction|RemoveSplashUI))))
    (:then_1
      (if (not (Variables|Default|GetbIsSplashScreenShowing))
        (CallFunction|WinCondition)))
    (:then_2
      (if (Variables|Default|GetbIsPlaying)
        (bind (_returnvalue_4 _abletospawn) (CallFunction|SpawnLimit))
        (if _abletospawn
          (bind _output_get (Variables|Default|SetSpawnTimer (- (Variables|Default|GetSpawnTimer) _returnvalue_3)))
          (if (<= _output_get 0.0)
            (bind _output_get_2 (Variables|Default|SetTypeToSpawn _returnvalue_4))
            (switch Utilities|FlowControl|Switch|SwitchonE_EnemyType _output_get_2
              (:NewEnumerator0
                (Default|CanSpawn _output "NewEnumerator0"))
              (:NewEnumerator1
                (Default|CanSpawn _output "NewEnumerator1")))
            (Variables|Default|SetSpawnTimer 5.0))
          (else
            (Variables|Default|SetSpawnTimer 5.0)))))))

(fn ConstructionScript)

(fn GetLevel
  (return (Variables|Default|GetLevel)))

(fn GetRound
  (return (Variables|Default|GetRound)))

(fn SpawnPlayer
  (bind _outactors (Actor|GetAllActorsOfClass "/Script/Engine.PlayerStart"))
  (bind _returnvalue (Game|SpawnActorfromClass "/Game/Blueprints/Characters/Player/Qbert/BP_Player.BP_Player_C" (Transformation|GetActorTransform (Utilities|Array|Get(acopy) _outactors)) "Undefined" 0 0))
  (bind _output_get (Variables|Default|SetPlayerRef _returnvalue))
  (Pawn|Possess (Game|GetPlayerController 0) _output_get)
  (Variables|Default|SetbIsPlaying true)
  (CallFunction|SetCam))

(fn CharacterDie
  (params (NextLevel :type Boolean))
  (bind _playerref (Variables|Default|GetPlayerRef))
  (Variables|Default|SetbIsPlaying false)
  (CallFunction|KillEnemys)
  (Utilities|IsValid _playerref
    (:Is%20Valid
      (Actor|DestroyActor _playerref)
      (CallFunction|SetCam)
      (if NextLevel
        _
        (else
          (bind _result (Math|Integer|DecrementInt (Variables|Default|GetLives))
            (:%20%20
              (bind _output_get (Variables|Default|SetLives _result))
              (if (< _output_get 0)
                (Variables|Default|SetLives 0)
                (LocalVariables|SetbIsGameOver true))
              (Default|UpdateLives (Variables|Default|GetGameUI) (Variables|Default|GetLives))))))
      (return (LocalVariables|GetbIsGameOver)))))

(fn DisplaySplashUI
  (Utilities|IsValid (Variables|Default|GetSplashUI)
    (:Is%20Valid
      _)
    (:Is%20Not%20Valid
      (bind _returnvalue (UserInterface|CreateWidget "/Game/UI/WBP_GameSplashScreen.WBP_GameSplashScreen_C"))
      (Variables|Default|SetSplashUI _returnvalue)))
  (Default|UpdateSplashRound (Variables|Default|GetSplashUI) (Variables|Default|GetRound))
  (Default|UpdateSplashLevel (Variables|Default|GetSplashUI) (+ (Variables|Default|GetLevel) 1))
  (UserInterface|Viewport|AddtoViewport (Variables|Default|GetSplashUI) 9999999)
  (Variables|Default|SetbIsPlaying false)
  (Variables|Default|SetSplashScreenTimer 5.0)
  (Variables|Default|SetbIsSplashScreenShowing true)
  (CallFunction|LevelUpdate)
  (Variables|Default|SetFinishTiles 0)
  (CallFunction|ResetPlatforms))

(fn RemoveSplashUI
  (Widget|RemovefromParent (Variables|Default|GetSplashUI))
  (Variables|Default|SetbIsSplashScreenShowing false)
  (CallFunction|SpawnPlayer))

(fn WinCondition
  (if (== (Utilities|Array|Length (Variables|/Game/Blueprints/Platform/BP_LevelMaker.BP_LevelMaker_C|GetPlatformArray (Variables|Default|GetLevelMaker))) (Variables|Default|GetFinishTiles))
    (bind _result (Math|Integer|IncrementInt (Variables|Default|GetRound))
      (:%20%20
        (bind _output_get (Variables|Default|SetRound _result))
        (if (> _output_get 3)
          (Variables|Default|SetRound 1)
          (bind _result_2 (Math|Integer|IncrementInt (Variables|Default|GetLevel))
            (:%20%20
              (Variables|Default|SetLevel _result_2))))
        (CallFunction|DisplaySplashUI)
        (CallFunction|CharacterDie true)))))

(fn ResetPlatforms
  (for _array_element (Variables|/Game/Blueprints/Platform/BP_LevelMaker.BP_LevelMaker_C|GetPlatformArray (Variables|Default|GetLevelMaker))
    (Variables|/Game/Blueprints/Platform/BP_Platform.BP_Platform_C|SetNextSprite _array_element true)
    (Default|ResetCurrentChange _array_element)))

(fn SetCam
  (Game|Player|SetViewTargetwithBlend (Game|GetPlayerController 0) (Variables|Default|GetLevelCamera) 0.0 "VTBlend_Linear" 0.0 false))

(fn KillEnemys
  (for _array_element (Variables|Default|GetCharacters)
    (if (not (Actor|ActorHasTag _array_element "Player"))
      (Actor|DestroyActor _array_element))))

(fn SpawnLimit
  (LocalVariables|SetNumberOfSlimes 0)
  (LocalVariables|SetNumberOfSnakes 0)
  (bind _outactors (Actor|GetAllActorsOfClass "/Game/Blueprints/Characters/Enemys/BP_Enemy.BP_Enemy_C"))
  (for _array_element _outactors
    (switch Utilities|FlowControl|Switch|SwitchonE_EnemyType (Variables|/Game/Blueprints/Characters/Enemys/BP_Enemy.BP_Enemy_C|GetEnemyType _array_element)
      (:NewEnumerator0
        (bind _result (Math|Integer|IncrementInt (LocalVariables|GetNumberOfSlimes))
          (:%20%20
            (LocalVariables|SetNumberOfSlimes _result))))
      (:NewEnumerator1
        (bind _result_2 (Math|Integer|IncrementInt (LocalVariables|GetNumberOfSnakes))
          (:%20%20
            (LocalVariables|SetNumberOfSnakes _result_2))))))
  (if (< (LocalVariables|GetNumberOfSnakes) (Variables|Default|GetMaxSnakeEnemy))
    (Variables|Default|SetTypeToSpawn "NewEnumerator1")
    (LocalVariables|SetbCanSpawn true)
    (elif (< (LocalVariables|GetNumberOfSlimes) (Variables|Default|GetMaxSlimeEnemys))
      (Variables|Default|SetTypeToSpawn "NewEnumerator0")
      (LocalVariables|SetbCanSpawn true)
      (else
        (LocalVariables|SetbCanSpawn false))))
  (return (Variables|Default|GetTypeToSpawn) (LocalVariables|GetbCanSpawn)))