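; Game mode for the Qbert main menu that sets up the menu UI and provides access to scoreboard save data.
; BeginPlay creates WBP_MainMenu, adds it to the viewport and hands it to BP_MenuConroller on player 0.
; SaveData loads the BP_ScoreBoardSave from its slot, or creates and saves a new one if none exists, then returns it.
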(event EventBeginPlay
  (bind _returnvalue (UserInterface|CreateWidget "/Game/UI/WBP_MainMenu.WBP_MainMenu_C"))
  (bind _output_get (Variables|Default|SetMainMEnu _returnvalue))
  (UserInterface|Viewport|AddtoViewport _output_get 0)
  (bind _asbp_menu_conroller (Utilities|Casting|CastToBP_MenuConroller (Game|GetPlayerController 0)))
  (Variables|/Game/Blueprints/BP_MenuConroller.BP_MenuConroller_C|SetMenuWidget _asbp_menu_conroller _output_get))

(fn ConstructionScript)

(fn SaveData
  (bind _returnvalue (SaveGame|DoesSaveGameExist (Variables|Default|GetSlot%20Name)))
  (if _returnvalue
    (bind _returnvalue_2 (SaveGame|LoadGamefromSlot (Variables|Default|GetSlot%20Name)))
    (bind _asbp_score_board_save (Utilities|Casting|CastToBP_ScoreBoardSave _returnvalue_2))
    (LocalVariables|SetSaveDataObject _asbp_score_board_save)
    (return (LocalVariables|GetSaveDataObject))
    (else
      (bind _returnvalue_3 (SaveGame|CreateSaveGameObject "/Game/Blueprints/Data/BP_ScoreBoardSave.BP_ScoreBoardSave_C"))
      (LocalVariables|SetSaveDataObject _returnvalue_3)
      (bind _returnvalue_4 (SaveGame|SaveGametoSlot _returnvalue_3 (Variables|Default|GetSlot%20Name)))
      (if _returnvalue_4
        (Development|PrintString "Sace Data Created")
        (return (LocalVariables|GetSaveDataObject))))))