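; Q*bert-style platform tile that changes sprite and awards score as the player lands on it.
; The Box trigger snaps overlapping actors above the tile, while the Floor trigger toggles grounded state on base characters.
; Each player landing, gated by a DoOnce reset on leaving, advances the level-based sprite and adds score scaled by level and round.
; Once changes reach the round number, the tile locks and increments the GameMode's finished-tile count.
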(event OnComponentBeginOverlap(Box)
  (params (OverlappedComponent :type Primitive%20Component%20Object%20Reference) (OtherActor :type Actor%20Object%20Reference) (OtherComp :type Primitive%20Component%20Object%20Reference) (OtherBodyIndex :type Integer) (bFromSweep :type Boolean) (SweepResult :type Hit%20Result%20Structure%20%28by%20ref%29))
  (bind _box (Variables|Default|GetBox))
  (bind _returnvalue (Transformation|GetWorldLocation _box))
  (bind (_x _y _z) (Math|Vector|BreakVector _returnvalue))
  (Transformation|SetActorLocation OtherActor (Math|Vector|MakeVector _x (+ _y 0.1) (+ _z 4.0)) true false))

(event OnComponentEndOverlap(Floor)
  (params (OverlappedComponent :type Primitive%20Component%20Object%20Reference) (OtherActor :type Actor%20Object%20Reference) (OtherComp :type Primitive%20Component%20Object%20Reference) (OtherBodyIndex :type Integer))
  (bind _gm (Variables|Default|GetGM))
  (bind _gm_2 (Variables|Default|GetGM))
  (bind _gm_3 (Variables|Default|GetGM))
  (bind _playerstate (Variables|Default|GetPlayerState))
  ;[1 1 1] Actor is jumping
  (Development|PrintString (Utilities|GetDisplayName OtherActor))
  (bind _asbp_base_character (Utilities|Casting|CastToBP_BaseCharacter OtherActor)
    (:then
      (Variables|/Game/Blueprints/Characters/BP_BaseCharacter.BP_BaseCharacter_C|SetIsGrounded _asbp_base_character false)
      (if (Actor|ActorHasTag OtherActor "Player")
        (Utilities|FlowControl|DoOnce false) ; enters at Reset
      ))
    (:CastFailed
      (Development|PrintString "Not BaseCharacter"))))

(event OnComponentBeginOverlap(Floor)
  (params (OverlappedComponent :type Primitive%20Component%20Object%20Reference) (OtherActor :type Actor%20Object%20Reference) (OtherComp :type Primitive%20Component%20Object%20Reference) (OtherBodyIndex :type Integer) (bFromSweep :type Boolean) (SweepResult :type Hit%20Result%20Structure%20%28by%20ref%29))
  (bind _gm (Variables|Default|GetGM))
  (bind _gm_2 (Variables|Default|GetGM))
  (bind _gm_3 (Variables|Default|GetGM))
  (bind _playerstate (Variables|Default|GetPlayerState))
  ;[1 1 1] Actor is Grounded
  (Development|PrintString (Utilities|GetDisplayName OtherActor))
  (bind _asbp_base_character (Utilities|Casting|CastToBP_BaseCharacter OtherActor)
    (:then
      (Variables|/Game/Blueprints/Characters/BP_BaseCharacter.BP_BaseCharacter_C|SetIsGrounded _asbp_base_character true)
      (if (and (Variables|Default|GetNextSprite) (Actor|ActorHasTag OtherActor "Player"))
        (Utilities|FlowControl|DoOnce false
          (:Completed
            (bind _result (Math|Integer|IncrementInt (Variables|Default|GetCurrentChangeTimes))
              (:%20%20
                (Variables|Default|SetCurrentChangeTimes _result)
                (Rendering|Components|Sprite|SetSprite (Variables|Default|GetPaperSprite) (Utilities|Array|Get(acopy) (Variables|/Game/Blueprints/Mode/QbertGameMode.QbertGameMode_C|GetLevelSprites _gm_2) (+ (* (Math|Integer|%(Integer) (Default|GetLevel _gm_2) 3) 4) (Variables|Default|GetCurrentChangeTimes))))
                ;[0.07193 1 0.05805] Scale Score to level and Round
                (Variables|/Game/Blueprints/NewPlayerState.NewPlayerState_C|SetCurrentScore _playerstate (+ (Variables|/Game/Blueprints/NewPlayerState.NewPlayerState_C|GetCurrentScore _playerstate) (* (Variables|Default|GetPoints) (* (+ (Variables|/Game/Blueprints/Mode/QbertGameMode.QbertGameMode_C|GetLevel _gm) 1) (Variables|/Game/Blueprints/Mode/QbertGameMode.QbertGameMode_C|GetRound _gm)))))
                (Default|UpdateScore (Variables|Default|GetGM))
                (if (>= (Variables|Default|GetCurrentChangeTimes) (Default|GetRound (Variables|Default|GetGM)))
                  ;[1 1 1] Makes it so tile can't change anymore and tells the gm more that a platform is complete
                  (Variables|Default|SetNextSprite false)
                  (bind _result_2 (Math|Integer|IncrementInt (Variables|/Game/Blueprints/Mode/QbertGameMode.QbertGameMode_C|GetFinishTiles _gm_3))
                    (:%20%20
                      (Variables|/Game/Blueprints/Mode/QbertGameMode.QbertGameMode_C|SetFinishTiles _gm_3 _result_2))))))))))
    (:CastFailed
      (Development|PrintString "Not BaseCharacter"))))

(event EventBeginPlay
  (bind _asnew_player_state (Utilities|Casting|CastToNewPlayerState (Variables|/Script/Engine.Controller|GetPlayerState (Game|GetPlayerController 0))))
  (Variables|Default|SetPlayerState _asnew_player_state)
  (bind _asqbert_game_mode (Utilities|Casting|CastToQbertGameMode (Game|GetGameMode)))
  (Variables|Default|SetGM _asqbert_game_mode))

(fn ConstructionScript)

(fn ResetCurrentChange
  (Variables|Default|SetCurrentChangeTimes 0))