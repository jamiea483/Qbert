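; LevelMaker is an actor that builds a triangular pyramid of Platform actors when play begins.
; SpawnPlatforms uses nested loops over rows and slots, with each successive row one platform wider, lower and slightly shifted in Y.
; Each row's start shifts half a step along X to keep the pyramid centered and staggered.
; The first and last slot of every row are left empty.
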(event Custom|MakeLevel
  (CallFunction|SpawnPlatforms))

(event EventBeginPlay
  (CallFunction|MakeLevel))

(event Collision|EventActorBeginOverlap
  (params (OtherActor :type Actor%20Object%20Reference)))

(event EventTick
  (params (DeltaSeconds :type Float%20%28single-precision%29)))

(fn ConstructionScript)

(fn SpawnPlatforms
  (for _index (range 0 (Variables|Default|GetRow))
    (bind _output_get (LocalVariables|SetLastSlotinRow (+ _index 2)))
    (LocalVariables|SetRowStartLocation (Math|Vector|MakeVector (Math|Conversions|ToFloat(Integer) (+ (* _index -16) -32)) (Math|Conversions|ToFloat(Integer) (* _index 2)) (Math|Conversions|ToFloat(Integer) (* _index -23))))
    (for _index_2 (range 0 _output_get)
      (if (or (== _index_2 0) (== _index_2 (LocalVariables|GetLastSlotinRow)))
        _
        (else
          (Game|SpawnActorfromClass "/Game/Blueprints/Platform/Platform.Platform_C" (Math|Transform|MakeTransform (LocalVariables|GetRowStartLocation)) "Undefined" 0 0)))
      (LocalVariables|SetRowStartLocation (+ (LocalVariables|GetRowStartLocation) "32.000000, 0, 0")))))