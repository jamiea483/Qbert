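; Level builder that spawns a stepped, pyramid-style layout of platforms and elevators and can tear it down.
; MakeLevel runs SpawnPlatforms, whose nested loops widen each descending, offset row and use BP_PlatformLastRow for the bottom one.
; The end slots of each row stay empty, except on the second-to-last row, which gets left and right elevators.
; Spawned platforms go into PlatformArray, which ClearLevel empties in reverse after destroying all elevators.
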(event Custom|MakeLevel
  (CallFunction|SpawnPlatforms))

(event Custom|Clear%20Level
  (bind _platformarray (Variables|Default|GetPlatformArray))
  (bind _outactors (Actor|GetAllActorsOfClass "/Game/Blueprints/Platform/BP_Elevator.BP_Elevator_C"))
  (for _array_element _outactors
    (Actor|DestroyActor _array_element))
  (bind (_arrayindex _arrayelement) (Utilities|Array|ReverseforEachLoop _platformarray)
    (:LoopBody
      (Actor|DestroyActor _arrayelement)
      (Utilities|Array|RemoveIndex _platformarray _arrayindex))))

(event EventBeginPlay)

(event Collision|EventActorBeginOverlap
  (params (OtherActor :type Actor%20Object%20Reference)))

(event EventTick
  (params (DeltaSeconds :type Float%20%28single-precision%29)))

(fn ConstructionScript)

(fn SpawnPlatforms
  ;[1 1 1] Row Start Position
  (LocalVariables|SetIndex 0)
  (for _index (range 0 (Variables|Default|GetRow))
    (bind _output_get (LocalVariables|SetLastSlotinRow (+ _index 2)))
    (LocalVariables|SetRowStartLocation (Math|Vector|MakeVector (Math|Conversions|ToFloat(Integer) (+ (* _index -16) -32)) (Math|Conversions|ToFloat(Integer) (* _index 2)) (Math|Conversions|ToFloat(Integer) (* _index -23))))
    (for _index_2 (range 0 _output_get)
      (if (or (== _index_2 0) (== _index_2 (LocalVariables|GetLastSlotinRow)))
        ;[1 1 1] Spawn 2 Elevators
        (if (== _index (- (Variables|Default|GetRow) 1))
          (if (== _index_2 0)
            (LocalVariables|SetbLocalOnLeft true)
            (else
              (LocalVariables|SetbLocalOnLeft false)))
          (Game|SpawnActorfromClass "/Game/Blueprints/Platform/BP_Elevator.BP_Elevator_C" (Math|Transform|MakeTransform (Math|Vector|MakeVector (.X (Math|Vector|BreakVector (.Location (Math|Transform|BreakTransform (Math|Transform|MakeTransform (LocalVariables|GetRowStartLocation)))))) (.Y (Math|Vector|BreakVector (.Location (Math|Transform|BreakTransform (Math|Transform|MakeTransform (LocalVariables|GetRowStartLocation)))))) (+ (.Z (Math|Vector|BreakVector (.Location (Math|Transform|BreakTransform (Math|Transform|MakeTransform (LocalVariables|GetRowStartLocation)))))) 7.0))) "Undefined" 0 (LocalVariables|GetbLocalOnLeft) 0))
        (else
          (if (== _index (Variables|Default|GetRow))
            (bind _returnvalue (Game|SpawnActorfromClass "/Game/Blueprints/Platform/BP_PlatformLastRow.BP_PlatformLastRow_C" (Math|Transform|MakeTransform (LocalVariables|GetRowStartLocation)) "Undefined" 0 "0.000000,0.000000,0.000000" 0))
            (LocalVariables|SetCurrentPlatform _returnvalue)
            (else
              (bind _returnvalue_2 (Game|SpawnActorfromClass "/Game/Blueprints/Platform/BP_Platform.BP_Platform_C" (Math|Transform|MakeTransform (LocalVariables|GetRowStartLocation)) "Undefined" 0 "0.000000,0.000000,0.000000" 0))
              (LocalVariables|SetCurrentPlatform _returnvalue_2)))
          (Utilities|Array|SetArrayElem (Variables|Default|GetPlatformArray) (LocalVariables|GetIndex) (LocalVariables|GetCurrentPlatform) true)
          (bind _result (Math|Integer|IncrementInt (LocalVariables|GetIndex))
            (:%20%20
              (LocalVariables|SetIndex _result)))))
      (LocalVariables|SetRowStartLocation (+ (LocalVariables|GetRowStartLocation) "32.000000, 0, 0")))))