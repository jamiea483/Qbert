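; Q*bert side elevator that carries the player to a point above the level, offset by its OnLeft side from BP_LevelMaker.
; Box overlap snaps and attaches the player, pauses play and starts a Tick countdown.
; When it expires, the GameMode kills enemies and the platform lerps to the target with growing alpha.
; On arrival it releases the player, triggers a jump down, resumes play, resets the tile location and destroys itself.
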(event OnComponentBeginOverlap(Box)
  (params (OverlappedComponent :type Primitive%20Component%20Object%20Reference) (OtherActor :type Actor%20Object%20Reference) (OtherComp :type Primitive%20Component%20Object%20Reference) (OtherBodyIndex :type Integer) (bFromSweep :type Boolean) (SweepResult :type Hit%20Result%20Structure%20%28by%20ref%29))
  (bind _asbp_player (Utilities|Casting|CastToBP_Player OtherActor))
  (Utilities|FlowControl|DoOnce false
    (:Completed
      (Variables|Default|SetPlayerRef _asbp_player)
      (Transformation|SetActorLocation _asbp_player (Transformation|GetWorldLocation (Variables|Default|GetBox)) false false)
      (Transformation|AttachComponentToComponent _asbp_player (Variables|Default|GetBox) "None" "SnapToTarget" "KeepWorld" "KeepWorld" true)
      (Variables|Default|SetbPlayerOnPlatform true)
      (Actor|Tick|SetActorTickEnabled true)
      (Variables|/Game/Blueprints/Mode/QbertGameMode.QbertGameMode_C|SetbIsPlaying (Variables|Default|GetGM) false)
      (Variables|/Game/Blueprints/Characters/BP_BaseCharacter.BP_BaseCharacter_C|SetIsGrounded (Variables|Default|GetPlayerRef) true))))

(event Custom|TranslateElevator
  (bind _self self)
  (bind _playerref (Variables|Default|GetPlayerRef))
  (bind _returnvalue (Transformation|GetActorLocation _self))
  (Transformation|SetActorLocation (Math|Vector|Lerp(Vector) _returnvalue (Variables|Default|GetTargetLocation) (Variables|Default|GetMoveTime)) false false)
  (if (Math|Vector|Equal(Vector) _returnvalue (Variables|Default|GetTargetLocation) 0.2)
    (Utilities|FlowControl|DoOnce false
      (:Completed
        (Transformation|DetachFromActor _playerref "KeepWorld" "KeepWorld" "KeepWorld")
        (Utilities|FlowControl|Delay 0.1)
        (Physics|SetSimulatePhysics (Variables|/Script/Engine.Character|GetCapsuleComponent _playerref) true)
        (Utilities|FlowControl|Delay 1.0)
        (if (Variables|Default|GetbOnLeft)
          (Default|ElevatorJumpDownRight _playerref)
          (else
            (Default|ElevatorJumpDownLeft _playerref)))
        (Variables|/Game/Blueprints/Mode/QbertGameMode.QbertGameMode_C|SetbIsPlaying (Variables|Default|GetGM) true)
        (Variables|/Game/Blueprints/Characters/BP_BaseCharacter.BP_BaseCharacter_C|SetTileLocation (Variables|Default|GetPlayerRef) "1.000000,1.000000, 0")
        (Actor|DestroyActor)))))

(event EventBeginPlay
  (bind _asqbert_game_mode (Utilities|Casting|CastToQbertGameMode (Game|GetGameMode)))
  (Variables|Default|SetGM _asqbert_game_mode)
  (bind _outactors (Actor|GetAllActorsOfClass "/Game/Blueprints/Platform/BP_LevelMaker.BP_LevelMaker_C"))
  (Variables|Default|SetLavelMakerRef (Utilities|Array|Get(acopy) _outactors))
  (if (Variables|Default|GetbOnLeft)
    (CallFunction|GetTargetLocation -1.0)
    (else
      (CallFunction|GetTargetLocation 1.0))))

(event EventTick
  (params (DeltaSeconds :type Float%20%28single-precision%29))
  (if (Variables|Default|GetbPlayerOnPlatform)
    (if (< (Variables|Default|GetStartMoveTimer) 0.0)
      (Utilities|FlowControl|Sequence
        (:then_0
          (Utilities|FlowControl|DoOnce false
            (:Completed
              (Default|KillEnemys (Variables|Default|GetGM)))))
        (:then_1
          (CallFunction|ElevatorLerpAlpha DeltaSeconds)
          (CallFunction|TranslateElevator)))
      (else
        (CallFunction|MoveTimer DeltaSeconds)))))

(fn ConstructionScript)

(fn GetTargetLocation
  (params (NewParam :type Float%20%28single-precision%29))
  (bind _lavelmakerref (Variables|Default|GetLavelMakerRef))
  (bind _returnvalue (Transformation|GetActorLocation _lavelmakerref))
  (bind (_x _y _z) (Math|Vector|BreakVector _returnvalue))
  (Variables|Default|SetTargetLocation (Math|Vector|MakeVector (+ _x (* NewParam 16.0)) (+ _y -2.0) (+ _z 3e+01))))

(fn StartMoving)

(fn MoveTimer
  (params (A :type Float%20%28single-precision%29))
  (Variables|Default|SetStartMoveTimer (- (Variables|Default|GetStartMoveTimer) (* A (Math|Float|MakeLiteralFloat 1.0))))
  (return))

(fn ElevatorLerpAlpha
  (params (A :type Float%20%28single-precision%29))
  (Variables|Default|SetMoveTime (+ (* A (Math|Float|MakeLiteralFloat (Variables|Default|GetMoveSpeed))) (Variables|Default|GetMoveTime)))
  (return))