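; KillZone is a box trigger for the Qbert game that reacts when the player or an enemy enters it.
; It caches the QbertGameMode on BeginPlay and asks it to restart the current level when an actor tagged Player overlaps the box.
; An overlapping BP_Enemy instead decrements its Spawner's EnemyLimit, and the enemy itself is not destroyed here.
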(event OnComponentBeginOverlap(Box)
  (params (OverlappedComponent :type Primitive%20Component%20Object%20Reference) (OtherActor :type Actor%20Object%20Reference) (OtherComp :type Primitive%20Component%20Object%20Reference) (OtherBodyIndex :type Integer) (bFromSweep :type Boolean) (SweepResult :type Hit%20Result%20Structure%20%28by%20ref%29))
  (if (Actor|ActorHasTag OtherActor "Player")
    (Default|RestarCurrenttLevel (Variables|Default|GetQbert%20Game%20Mode))
    (else
      (bind _asbp_enemy (Utilities|Casting|CastToBP_Enemy OtherActor))
      (Variables|/Game/Blueprints/Characters/Enemys/BP_EnemySpawner.BP_EnemySpawner_C|SetEnemyLimit (Variables|/Game/Blueprints/Characters/Enemys/BP_Enemy.BP_Enemy_C|GetSpawner _asbp_enemy) (- (Variables|/Game/Blueprints/Characters/Enemys/BP_EnemySpawner.BP_EnemySpawner_C|GetEnemyLimit (Variables|/Game/Blueprints/Characters/Enemys/BP_Enemy.BP_Enemy_C|GetSpawner _asbp_enemy)) 1)))))

(event EventBeginPlay
  (bind _asqbert_game_mode (Utilities|Casting|CastToQbertGameMode (Game|GetGameMode)))
  (Variables|Default|SetQbert%20Game%20Mode _asqbert_game_mode))

(fn ConstructionScript)